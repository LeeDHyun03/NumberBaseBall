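; Player controller for a multiplayer turn-based number baseball game played through a chat widget.
; Committed text goes to the game mode as chat, or as a guess when it is a slash plus three digits on the player's turn, with three chances.
; Game-mode broadcasts return scores, turns and outcomes to the chat log.
; Replicated MyTurn starts or clears the local countdown, whose expiry adds an out.
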(event Custom|GotBroadcastNumber_Event
  (params (UserID :type String) (Ball :type Integer) (Strike :type Integer) (Count :type Integer))
  ;[0.15 0.15 0.15 0.5] Broadcast Number
  (if (Ability|HasAuthority)
    (CallFunction|SendtoWidgetEvent (Utilities|String|Append "B: " (Utilities|String|ToString(Integer) Ball) "   " "S: " (Utilities|String|ToString(Integer) Strike) "   " "O: " (Utilities|String|ToString(Integer) Count) "   " "Num: " (Variables|Default|GetNumber)) UserID)))

(event Custom|OnLoginWithID_Event
  (params (User%20ID :type String))
  ;[0.15 0.15 0.15 0.5] OnLogin
  (if (Ability|HasAuthority)
    (Variables|Default|SetUserID User%20ID)))

(event Custom|StartTimer
  (bind _returnvalue (Utilities|Time|SetTimerbyEvent (EventDispatchers|CreateEvent :!event Custom|CountDownTimer) 1.0 true))
  (Variables|Default|SetCountDownHandle _returnvalue)
  (Variables|Default|SetCurrentTime (Variables|Default|GetMaxTime))
  (CallFunction|SendtoChangedTurnforGameModeEvent))

(event Custom|CountDownTimer
  (bind _result (Math|Integer|DecrementInt (Variables|Default|GetCurrentTime))
    (:%20%20
      (Default|TimerEventEvent (Variables|Default|GetWidget) _result)
      (if (== (Variables|Default|GetCurrentTime) 0)
        (Utilities|Time|ClearandInvalidateTimerbyHandle (Variables|Default|GetCountDownHandle))
        (CallFunction|Time'sUpEvent)))))

(event Custom|GotBroadcastTime'sUp_Event
  (params (UserID :type String))
  (if (Ability|HasAuthority)
    (CallFunction|SendtoWidgetEvent (Utilities|String|Append UserID " Time's Up. Add 1 Out") "Server")))

(event Custom|Time's%20Up_Event
  (Math|Integer|IncrementInt (Variables|Default|GetCount)
    (:%20%20
      (bind _asbp_number_base_ball_game_mode (Utilities|Casting|CastToBP_NumberBaseBallGameMode (Game|GetGameMode)))
      (Default|Time'sUpEvent _asbp_number_base_ball_game_mode (Variables|Default|GetUserID) (Variables|Default|GetCount)))))

(event Custom|GotBroadcastChangedTurn_Event
  (params (UserID :type String))
  (if (Ability|HasAuthority)
    (CallFunction|SendtoWidgetEvent (Utilities|String|Append UserID " Turn") "Server")))

(event Custom|SendToChangedTurnForGameMode_Event
  (bind _asbp_number_base_ball_game_mode (Utilities|Casting|CastToBP_NumberBaseBallGameMode (Game|GetGameMode)))
  (Default|GotChangedTurnfromClientEvent _asbp_number_base_ball_game_mode (Variables|Default|GetUserID)))

(event Custom|OnSendCommitTextToServer_Event
  (params (Text :type String))
  ;[0.15 0.15 0.15 0.5] Distinguish what Commit Message is Text or Number
  (Variables|Default|SetCommitText Text)
  (bind _asbp_number_base_ball_game_mode (Utilities|Casting|CastToBP_NumberBaseBallGameMode (Game|GetGameMode)))
  (if (Variables|/Game/Blueprints/BP_NumberBaseBallGameMode.BP_NumberBaseBallGameMode_C|GetbIsStart _asbp_number_base_ball_game_mode)
    (if (Variables|Default|GetMyTurn)
      (if (Utilities|Enum|Equal(Enum) (Utilities|String|Left (Variables|Default|GetCommitText) 1) "/")
        (bind _output_get (Variables|Default|SetCommitTextArray (Utilities|String|GetCharacterArrayfromString (Variables|Default|GetCommitText))))
        (Utilities|Array|RemoveIndex _output_get)
        (if (== (Utilities|Array|Length (Variables|Default|GetCommitTextArray)) 3)
          (bind _array_element (Utilities|Array|ForEachLoopwithBreak (Variables|Default|GetCommitTextArray) :!label _label)
            (:LoopBody
              (bind _output_get_2 (Variables|Default|SetIsNum (Class|KismetStringLibrary|IsNumeric _array_element)))
              (if _output_get_2
                (Utilities|Array|Add (Variables|Default|GetMyNumber) (Math|Conversions|ToInteger(Byte) _array_element))
                (else
                  (goto _label Break))))
            (:Completed
              (if (Variables|Default|GetIsNum)
                (if (< (Variables|Default|GetCount) 3)
                  (bind _result (Math|Integer|IncrementInt (Variables|Default|GetCount))
                    (:%20%20
                      (Default|GotIndexFormClientEvent _asbp_number_base_ball_game_mode (Variables|Default|GetMyNumber) _result (Variables|Default|GetUserID))
                      (Variables|Default|SetIsNum true :!label _label_2)
                      (Utilities|Array|Clear (Variables|Default|GetMyNumber))
                      (Variables|Default|SetMyNumber (Utilities|Array|MakeArray))))
                  (else
                    (CallFunction|SendtoWidgetEvent "You Don't Have Chance" "Server")))
                (else
                  (Default|GotTextFormClientEvent _asbp_number_base_ball_game_mode (Variables|Default|GetCommitText) (Variables|Default|GetUserID) :!label _label_3)
                  (goto _label_2)))))
          (else
            (goto _label_3)))
        (else
          (goto _label_3)))
      (else
        (goto _label_3)))
    (else
      (goto _label_3))))

(event Custom|GotBroadcastText_Event
  (params (Text :type String) (UserID :type String))
  ;[0.15 0.15 0.15 0.5] Broadcast Text
  (if (Ability|HasAuthority)
    (CallFunction|SendtoWidgetEvent Text UserID)))

(event Custom|GotBroadcastClear_Event
  (params (User%20ID :type String))
  ;[0.15 0.15 0.15 0.5] Broadcast Clear
  (if (Ability|HasAuthority)
    (CallFunction|SendtoWidgetEvent (Utilities|String|Append "Success!  " "Answer: " (Variables|Default|GetNumber)) User%20ID)
    (Variables|Default|SetCount 0)))

(event Custom|GotBroadcastFailed_Event
  (params (User%20ID :type String))
  ;[0.15 0.15 0.15 0.5] Broadcast Failed
  (if (Ability|HasAuthority)
    (CallFunction|SendtoWidgetEvent "is Failed!!" User%20ID)))

(event Custom|GotBroadcastAllPlayerFailed_Event
  ;[0.15 0.15 0.15 0.5] Broadcast All Player Failed
  (if (Ability|HasAuthority)
    (CallFunction|SendtoWidgetEvent "All Player is Failed. Restart Game!" "Server")
    (Variables|Default|SetNumber "")
    (Variables|Default|SetCount 0)))

(event Custom|SendToWidget_Event
  (params (Text :type String) (UserID :type String))
  ;[0.15 0.15 0.15 0.5] Add To Text for Widget
  (Default|AddChatLogEvent (Variables|Default|GetWidget) Text UserID))

(event Custom|GotOtherPlayerNumber_Event
  (params (PlayerNumber :type Array%20of%20Integers))
  (if (Ability|HasAuthority)
    (Variables|Default|SetNumber "")
    (for _array_element PlayerNumber
      (Variables|Default|SetNumber (Utilities|String|Append (Variables|Default|GetNumber) (Utilities|String|ToString(Integer) _array_element))))))

(event EventBeginPlay
  ;[0.15 0.15 0.15 0.5] If client, create Widget
  (if (Pawn|IsLocalController)
    (bind _returnvalue (UserInterface|CreateWidget "/Game/WBP_Chat.WBP_Chat_C"))
    (bind _output_get (Variables|Default|SetWidget _returnvalue))
    (UserInterface|Viewport|AddtoViewport _output_get 0)
    (EventDispatchers|BindEventtoOnCommitText (Variables|Default|GetWidget) (EventDispatchers|CreateEvent :!event Custom|OnSendCommitTextToServer_Event))
    (Variables|Default|SetbShowMouseCursor true)
    (Input|SetInputModeUIOnly (Game|GetPlayerController 0) (Variables|Default|GetWidget) "DoNotLock" false)))

(fn ConstructionScript)

(fn OnRepMyTurn
  (if (and (Variables|Default|GetMyTurn) (Pawn|IsLocalController))
    (CallFunction|StartTimer)
    (else
      (Utilities|Time|ClearandInvalidateTimerbyHandle (Variables|Default|GetCountDownHandle)))))